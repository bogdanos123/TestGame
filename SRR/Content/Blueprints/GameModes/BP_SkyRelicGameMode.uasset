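; Game mode for a relic-collecting game that sets objective text by level name and handles win and loss.
; Level 02 and Level 03 start a looping one-second countdown that pauses the game and shows the game over screen at zero.
; AddRelic counts pickups and, at the required total, unlocks the first BP_Portal found, or shows the win screen if none exists.
; Both end screens switch input to UI only.
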(event EventBeginPlay
  (bind _returnvalue (Game|GetCurrentLevelName true))
  (switch string _returnvalue
    (:ThirdPersonMap
      (Variables|Default|SetObjectiveText "Collect 5 relics, unlock and reach the portal.")
      (Variables|Default|SetShowTimer false))
    (:Level_02
      (Variables|Default|SetObjectiveText "Collect 5 relics before time runs out.")
      (Variables|Default|SetShowTimer true :!label _label)
      (Variables|Default|SetTimeLeft 60)
      (Utilities|Time|SetTimerbyFunctionName 0 "Update Timer" 1.0 true))
    (:Level_03
      (Variables|Default|SetObjectiveText "Watch your step!")
      (goto _label))))

(fn ConstructionScript)

(fn AddRelic
  (Variables|Default|SetRelicsCollected (+ (Variables|Default|GetRelicsCollected) 1))
  (if (>= (Variables|Default|GetRelicsCollected) (Variables|Default|GetRequiredRelics))
    (bind _outactors (Actor|GetAllActorsOfClass "/Game/Blueprints/Interactables/BP_Portal.BP_Portal_C"))
    (if (> (Utilities|Array|Length _outactors) 0)
      (Variables|/Game/Blueprints/Interactables/BP_Portal.BP_Portal_C|SetIsUnlocked (Utilities|Array|Get(acopy) _outactors) true)
      (else
        (CallFunction|ShowWinScreen)))))

(fn ShowGameOverScreen
  (bind _returnvalue (Game|GetPlayerController 0))
  (bind _returnvalue_2 (UserInterface|CreateWidget "/Game/Blueprints/UI/WBP_GameOverScreen.WBP_GameOverScreen_C"))
  (UserInterface|Viewport|AddtoViewport _returnvalue_2 0)
  (Game|SetGamePaused true)
  (Variables|/Script/Engine.PlayerController|SetbShowMouseCursor _returnvalue true)
  (Input|SetInputModeUIOnly _returnvalue 0 "DoNotLock" false))

(fn UpdateTimer
  (if (> (Variables|Default|GetTimeLeft) 0)
    (Variables|Default|SetTimeLeft (- (Variables|Default|GetTimeLeft) 1))
    (if (<= (Variables|Default|GetTimeLeft) 0)
      (CallFunction|ShowGameOverScreen))))

(fn ShowWinScreen
  (bind _returnvalue (Game|GetPlayerController 0))
  (bind _returnvalue_2 (UserInterface|CreateWidget "/Game/Blueprints/UI/WBP_WinScreen.WBP_WinScreen_C"))
  (UserInterface|Viewport|AddtoViewport _returnvalue_2 0)
  (Variables|/Script/Engine.PlayerController|SetbShowMouseCursor _returnvalue true)
  (Input|SetInputModeUIOnly _returnvalue 0 "DoNotLock" false))