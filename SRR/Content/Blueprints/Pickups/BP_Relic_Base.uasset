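; Base relic pickup actor that the player character collects to add a relic to the Sky Relic game mode.
; A sphere overlap with the third-person character calls AddRelic on the game mode, plays the pickup sound at world origin and destroys the actor.
; Each tick, a sine of game time, scaled by float speed and height, bobs the actor vertically around its BeginPlay location.
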(event OnComponentBeginOverlap(Sphere)
  (params (OverlappedComponent :type Primitive%20Component%20Object%20Reference) (OtherActor :type Actor%20Object%20Reference) (OtherComp :type Primitive%20Component%20Object%20Reference) (OtherBodyIndex :type Integer) (bFromSweep :type Boolean) (SweepResult :type Hit%20Result%20Structure%20%28by%20ref%29))
  ;[1 1 1] Relic Pickup Logic
  (Utilities|Casting|CastToBP_ThirdPersonCharacter OtherActor)
  (bind _asbp_sky_relic_game_mode (Utilities|Casting|CastToBP_SkyRelicGameMode (Game|GetGameMode)))
  (Default|AddRelic _asbp_sky_relic_game_mode)
  (Audio|PlaySoundatLocation "/Game/Assets/PickUpSound.PickUpSound" "0, 0, 0" "0, 0, 0" 1.0 1.0 0.0 0 0 0 0)
  (Actor|DestroyActor self))

(event EventBeginPlay
  (Variables|Default|SetStartLocation (Transformation|GetActorLocation)))

(event EventTick
  (params (DeltaSeconds :type Float%20%28single-precision%29))
  (Transformation|SetActorLocation (+ (Math|Vector|MakeVector 0.0 0.0 (* (Math|Trig|Sin(Radians) (* (Utilities|Time|GetGameTimeinSeconds) (Variables|Default|GetFloatSpeed))) (Variables|Default|GetFloatHeight))) (Variables|Default|GetStartLocation)) false false))

(fn ConstructionScript)